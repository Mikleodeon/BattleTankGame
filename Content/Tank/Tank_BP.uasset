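; Player-controllable tank Blueprint that binds input for camera aim, track movement and firing.
; BeginPlay hands the turret and barrel components to the tank through setter calls.
; Aim axes rotate separate spring-arm yaw and pitch components, with elevation inverted and halved.
; Movement supports direct per-track throttles and fly-by-wire intent through TankMoveComponent, where forward and backward axes both feed IntendMoveForward.
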(event EventBeginPlay
  ;[1 1 1] setup for components
  (Class|Tank|SetTurretReference (Variables|Default|GetTankTurret))
  (Class|Tank|SetBarrelReference (Variables|Default|GetTankBarrel)))

(event Collision|EventActorBeginOverlap
  (params (OtherActor :type Actor%20Object%20Reference)))

(event Input|ActionEvents|InputActionFire
  (params (Key :type Key%20Structure))
  ;[1 1 1] Input Binding
  ;;[1 1 1] Fire
  (:Pressed
    (Class|Tank|Fire)))

(event Input|AxisEvents|InputAxisAimYaw
  (params (AxisValue :type Float%20%28single-precision%29))
  ;[1 1 1] Input Binding
  ;;[1 1 1] Camera
  (Transformation|AddLocalRotation (Variables|Default|GetSpringArm_Yaw) (Math|Rotator|MakeRotator 0.0 0.0 AxisValue) false false))

(event Input|AxisEvents|InputAxisLeftThrottle
  (params (AxisValue :type Float%20%28single-precision%29))
  ;[1 1 1] Input Binding
  ;;[1 1 1] Movement
  ;;;[1 1 1] Direct
  (Class|TankTrack|SetThrottle (Variables|Default|GetLeftTankTrack) (Variables|Default|GetforceNewtons) AxisValue))

(event Input|AxisEvents|InputAxisMoveForward
  (params (AxisValue :type Float%20%28single-precision%29))
  ;[1 1 1] Input Binding
  ;;[1 1 1] Movement
  ;;;[1 1 1] Fly by Wire
  (Class|TankMovementComponent|IntendMoveForward (Variables|Default|GettankMoveComponent) AxisValue))

(event Input|AxisEvents|InputAxisMoveBackward
  (params (AxisValue :type Float%20%28single-precision%29))
  ;[1 1 1] Input Binding
  ;;[1 1 1] Movement
  ;;;[1 1 1] Fly by Wire
  (Class|TankMovementComponent|IntendMoveForward (Variables|Default|GettankMoveComponent) AxisValue))

(event Input|AxisEvents|InputAxisAimElevation
  (params (AxisValue :type Float%20%28single-precision%29))
  ;[1 1 1] Input Binding
  ;;[1 1 1] Camera
  (Transformation|AddLocalRotation (Variables|Default|GetSpringArm_Pitch) (Math|Rotator|MakeRotator 0.0 (* AxisValue -0.5) 0.0) false false))

(event Input|AxisEvents|InputAxisRightThrottle
  (params (AxisValue :type Float%20%28single-precision%29))
  ;[1 1 1] Input Binding
  ;;[1 1 1] Movement
  ;;;[1 1 1] Direct
  (Class|TankTrack|SetThrottle (Variables|Default|GetRightTankTrack) (Variables|Default|GetforceNewtons) AxisValue))

(fn ConstructionScript)