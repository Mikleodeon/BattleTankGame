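; Tank controller Blueprint that creates the PlayerUI widget and adds it to the viewport on BeginPlay.
; It also holds an unwired crosshair trace prototype that never runs.
; That prototype deprojects a screen point slightly below center and line-traces on Visibility from the camera along that direction, with persistent debug drawing and a debug print.
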(event EventBeginPlay
  ;[1 1 1] Initialize PlayerUI
  (bind _returnvalue (UserInterface|CreateWidget "/Game/UI/PlayerUI.PlayerUI_C"))
  (UserInterface|Viewport|AddtoViewport _returnvalue 0))

(fn ConstructionScript)